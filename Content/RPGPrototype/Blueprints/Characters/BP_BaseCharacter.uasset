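; BP_BaseCharacter is a base character Blueprint that handles melee-style attacks, taking damage and death for the RPG prototype.
; Attack line-traces forward by AttackLength and damages the hit actor, while AIAttack plays a random attack montage, blocking re-entry until it finishes.
; Incoming damage goes to HealthComponent and plays a random hit montage.
; HealthComponent's OnDeath disables capsule collision and ragdolls the mesh.
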(event `self.HealthComponent.OnDeath`
  (bind _mesh (`self.Mesh`))
  (`PrimitiveComponent.SetCollisionEnabled` (`self.CapsuleComponent`) "NoCollision")
  (`PrimitiveComponent.SetSimulatePhysics` _mesh true)
  (`PrimitiveComponent.SetCollisionEnabled` _mesh "QueryAndPhysics"))

(event `Attack`
  (bind _returnvalue (`self.K2_GetActorLocation`))
  (bind (_outhit _returnvalue_2) (`KismetSystemLibrary.LineTraceSingle` _returnvalue (+ _returnvalue (* (`self.GetActorForwardVector`) (`self.AttackLength`))) "TraceTypeQuery1"))
  (if _returnvalue_2
    (`GameplayStatics.ApplyDamage` (`.HitActor` (`GameplayStatics.BreakHitResult` _outhit)) (`self.Damage`))))

(event `self.ReceiveAnyDamage`
  (params (Damage :type "Float (single-precision)") (DamageType :type "DamageType Object Reference") (InstigatedBy :type "Controller Object Reference") (DamageCauser :type "Actor Object Reference"))
  (`/Game/RPGPrototype/Blueprints/Components/BPC_Health.ApplyDamage` (`self.HealthComponent`) Damage)
  (bind _animation_result (`self.GetRandomAnimation` (`self.HitAnimations`)))
  (`self.PlayAnimMontage` _animation_result))

(event `AIAttack`
  (bind _attackspeed (`self.AttackSpeed`))
  (if (not (`self.IsAttack`))
    (bind _animation_result (`self.GetRandomAnimation` (`self.AttackAnimations`)))
    (set `self.IsAttack` true)
    (bind _returnvalue (`self.PlayAnimMontage` _animation_result _attackspeed))
    (`KismetSystemLibrary.Delay` (/ _returnvalue _attackspeed))
    (set `self.IsAttack` false)))

(fn `GetRandomAnimation`
  (params (Animations :type "Array of AnimMontage Object Reference"))
  (returns (`Animation Result` :type "AnimMontage Object Reference"))
  (return (`|GetArrayItem` Animations (`KismetMathLibrary.RandomInteger` (`KismetArrayLibrary.Array_Length` Animations)))))

(fn `UserConstructionScript`)