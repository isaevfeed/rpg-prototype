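; Enemy spawner actor that keeps the level stocked with a configured enemy class up to a target count.
; On BeginPlay it starts a looping millisecond-interval timer that calls Spawn.
; Spawn counts all actors of that class in the world and, while below the target, spawns one per call.
; Each spawn point is randomized from the Box component's scaled X/Y extents and transformed to the box's world position and rotation.
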(event `self.ReceiveBeginPlay`
  (`KismetSystemLibrary.K2_SetTimer` null "Spawn" 0.001 true))

(fn `CheckEnemyCount`
  (returns (StopSpawn :type Boolean))
  (bind _outactors (`GameplayStatics.GetAllActorsOfClass` (`self.EnemyClass`)))
  (return (>= (`KismetArrayLibrary.Array_Length` _outactors) (`self.CountOfEnemies`))))

(fn `Spawn`
  (bind _box (`self.Box`))
  (bind (_returnvalue_x _returnvalue_y) (`KismetMathLibrary.BreakVector` (`BoxComponent.GetScaledBoxExtent` _box)))
  (bind (_returnvalue_location _returnvalue_rotation) (`KismetMathLibrary.BreakTransform` (`SceneComponent.K2_GetComponentToWorld` _box)))
  (bind _stopspawn (`self.CheckEnemyCount`))
  (if (not _stopspawn)
    (`|SpawnActorFromClass` (`self.EnemyClass`) (`KismetMathLibrary.MakeTransform` (`KismetMathLibrary.TransformLocation` (`KismetMathLibrary.MakeTransform` _returnvalue_location _returnvalue_rotation) (`KismetMathLibrary.RandomPointInBoundingBox` (0.0 0.0 0.0) (`KismetMathLibrary.MakeVector` (`KismetMathLibrary.RandomFloatInRange` 0.0 _returnvalue_x) (`KismetMathLibrary.RandomFloatInRange` 0.0 _returnvalue_y))))) "Undefined" "OverrideRootScale" null null)))

(fn `UserConstructionScript`)