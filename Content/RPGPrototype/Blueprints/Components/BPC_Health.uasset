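; BPC_Health is a health component that tracks an owner's current and maximum health in the RPG prototype.
; BeginPlay fills health to maximum, while healing and damage functions clamp the value and fire a health-changed dispatcher.
; Damage that drops health to zero fires a death dispatcher, guarded by a DoOnce that is never reset.
; Getters expose current health, health percentage and dead state.
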(event `self.ReceiveBeginPlay`
  (set `self.Health` (`self.MaxHealth`))
  (`self.OnHealthChanged`))

(fn `AddHealth`
  (params (HealthAmount :type "Float (double-precision)"))
  (set `self.Health` (`KismetMathLibrary.FMin` (+ HealthAmount (`self.Health`)) (`self.MaxHealth`)))
  (`self.OnHealthChanged`))

(fn `ApplyDamage`
  (params (Damage :type "Float (double-precision)"))
  (bind _output_get (set `self.Health` (`KismetMathLibrary.FMax` (- (`self.Health`) Damage))))
  (`self.OnHealthChanged`)
  (if (<= _output_get 0.0)
    (`/Engine/EditorBlueprintResources/StandardMacros.DoOnce` false
      (:`Completed`
        (`self.OnDeath`)))))

(fn `GetHealth`
  (returns (Health :type "Float (double-precision)"))
  (return (`self.Health`)))

(fn `GetHealthPercent`
  (returns (Percent :type "Float (double-precision)"))
  (return (/ (`self.Health`) (`self.MaxHealth`))))

(fn `IsDead`
  (returns (IsDead :type Boolean))
  (return (== (`self.Health`) 0.0)))